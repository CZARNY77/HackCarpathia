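; Pickup actor that shows a text prompt and hands itself to the player character when its trigger is overlapped.
; On BeginPlay it hides the text and caches the player as BP_My_Player.
; Trigger overlaps toggle the text and a PlayerNear flag without checking the overlapping actor, and entering calls PickUp on the cached player.
; DestroyPickUp destroys the actor but is not called within this Blueprint.
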(event `self.ReceiveBeginPlay`
  (`SceneComponent.SetVisibility` (`self.TextRender`) false false)
  (bind _asbp_my_player (cast `/Game/Blueprints/BP_My_Player` (`GameplayStatics.GetPlayerCharacter` 0)))
  (bind _output_get (set `self.Player` _asbp_my_player)))

(event `self.trigger.OnComponentBeginOverlap`
  (params (OverlappedComponent :type "PrimitiveComponent Object Reference") (OtherActor :type "Actor Object Reference") (OtherComp :type "PrimitiveComponent Object Reference") (OtherBodyIndex :type Integer) (bFromSweep :type Boolean) (SweepResult :type "HitResult Structure (by ref)"))
  (set `self.player near` true)
  (`SceneComponent.SetVisibility` (`self.TextRender`) true false)
  (`/Game/Blueprints/BP_My_Player.PickUp` (stale `self.ReceiveBeginPlay` _output_get) self))

(event `self.trigger.OnComponentEndOverlap`
  (params (OverlappedComponent :type "PrimitiveComponent Object Reference") (OtherActor :type "Actor Object Reference") (OtherComp :type "PrimitiveComponent Object Reference") (OtherBodyIndex :type Integer))
  (set `self.player near` false)
  (`SceneComponent.SetVisibility` (`self.TextRender`) false false))

(fn `DestroyPickUp`
  (`self.K2_DestroyActor`))

(fn `UserConstructionScript`)