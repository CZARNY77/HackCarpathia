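; AI-driven NPC that the player talks to by voice to take on and turn in a quest.
; Recorded microphone audio is exported to WAV, transcribed by OpenAI, then sent with the running chat log to GPT-3.5.
; Replies are scanned for trigger phrases that add or complete quests through the game mode's QuestManager, with completion prompting a congratulation.
; Name label visibility toggles by event; TextToSound is an empty stub.
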(event `self.ReceiveBeginPlay`
  (`OpenAIUtils.setUseOpenAIApiKeyFromEnvironmentVars` true)
  (bind _asbp_hack_carpathia_game_mode_base (cast `/Game/Blueprints/BP_HackCarpathiaGameModeBase` (`GameplayStatics.GetGameMode`)))
  (set `self.QuestManager` (`HackCarpathiaGameModeBase.QuestManagerInstance` _asbp_hack_carpathia_game_mode_base))
  (bind _asbp_my_player (cast `/Game/Blueprints/BP_My_Player` (`GameplayStatics.GetPlayerCharacter` 0)))
  (set `self.Player` _asbp_my_player)
  (`SceneComponent.SetVisibility` (`self.Name`) false false))

(event `NameVisibllityOn`
  (`SceneComponent.SetVisibility` (`self.Name`) true false))

(event `StartRecording`
  ;[1 1 1] Recording
  (`SynthComponent.Start` (`self.AudioCapture`))
  (`KismetSystemLibrary.PrintString` "Start")
  (`AudioMixerBlueprintLibrary.StartRecordingOutput` 1.0 (`self.MySubmix`)))

(event `NameVisibllityOff`
  (`SceneComponent.SetVisibility` (`self.Name`) false false))

(event `StopRecording`
  ;[1 1 1] Recording
  (`SynthComponent.Stop` (`self.AudioCapture`))
  (`AudioMixerBlueprintLibrary.StopRecordingOutput` "WavFile" (`self.FileName`) "" (`self.MySubmix`) null)
  (add `SoundSubmix.OnSubmixRecordedFileDone` (`self.MySubmix`) (delegate `SoundToText`)))

(event `SoundToText`
  (params (ResultingSoundWave :type "SoundWave Object Reference"))
  ;[1 1 1] Sound To Text
  (`KismetSystemLibrary.PrintString` "Konwertuje")
  (bind (_transcription _errormessage _success) (`OpenAICallTranscriptions.OpenAICallTranscriptions` (`self.FileName`))
    (:`Finished`
      (if _success
        (`KismetSystemLibrary.LogString` (`KismetStringLibrary.Concat_StrStr` "USER: " _transcription))
        (`self.SendPrompt` (make `ChatLog` "USER" _transcription))
        (else
          (`KismetSystemLibrary.PrintString` _errormessage))))))

(event `SendPrompt`
  (params (ChatLog :type "ChatLog Structure"))
  ;[1 1 1] Send Prompt
  (`KismetArrayLibrary.Array_Add` (`self.ChatLog`) ChatLog)
  (bind (_message _errormessage _success) (`OpenAICallChat.OpenAICallChat` (make `ChatSettings` "GPT_3_5_TURBO" (`self.ChatLog`) 0.7 150))
    (:`Finished`
      (if _success
        (bind _message_2 (break `ChatCompletion` _message))
        (`KismetArrayLibrary.Array_Add` (`self.ChatLog`) _message_2)
        (bind (_role _content) (break `ChatLog` _message_2))
        (`KismetSystemLibrary.LogString` (`KismetStringLibrary.Concat_StrStr` "ASSISTANT: " _content))
        (`self.ContextDetection` _content)
        (else
          (`KismetSystemLibrary.PrintString` _errormessage))))))

(event `AddSystemLog`
  (params (Prompt :type String))
  (`KismetArrayLibrary.Array_Add` (`self.ChatLog`) (make `ChatLog` "SYSTEM" Prompt)))

(event `TextToSound`)

(fn `AddQuest`
  (bind _questmanager (`self.QuestManager`))
  (`KismetSystemLibrary.LogString` "Biore questa")
  (if (not (`KismetSystemLibrary.IsValid` (`self.InstanceQuest`)))
    (set `QuestManager.QuestClass` (`self.Quest`) _questmanager)
    (bind _returnvalue (`QuestManager.AddQuest` _questmanager))
    (set `self.InstanceQuest` _returnvalue)
    (`/Game/Blueprints/BP_My_Player.CheatWiatrak` (`self.Player`))
    (`KismetSystemLibrary.LogString` "dodałem questa")))

(fn `CompletedQuest`
  (params (QuestID :type Name))
  (locals (ID :type Name))
  (set `local.ID` QuestID)
  (`KismetSystemLibrary.LogString` "Konczmy?")
  (if (`KismetSystemLibrary.IsValid` (`self.InstanceQuest`))
    (if (`QuestManager.CanReturnQuest` (`self.QuestManager`) (`local.ID`))
      (`QuestManager.CompletedQuest` (`self.QuestManager`) (`local.ID`))
      (`self.SendPrompt` (make `ChatLog` "SYSTEM" (`BlueprintMapLibrary.Map_Find` (`self.Promps`) "Gratulations")))
      (`/Game/Blueprints/BP_My_Player.ItemsOff` (`self.Player`) (`local.ID`))
      (`KismetSystemLibrary.LogString` "Zadanie ukonczone")
      (else
        (`KismetSystemLibrary.LogString` "Jeszcze nie ukonczyles zadania")))
    (else
      (`KismetSystemLibrary.LogString` "Jeszcze nie rozpoczeles zadania, ale czy masz potrzebne itemki"))))

(fn `ContextDetection`
  (params (Content :type String))
  (locals (Contents :type "Array of String") (CurrentContent :type String))
  (set `local.CurrentContent` Content)
  (for (_array_element _array_index) (`local.Contents`)
    (if (`KismetStringLibrary.Contains` (`local.CurrentContent`) _array_element)
      (switch `int` _array_index
        (:`0`
          (`self.AddQuest` :!label _label))
        (:`1`
          (goto _label))
        (:`2`
          (goto _label))
        (:`3`
          (goto _label))
        (:`4`
          (goto _label))
        (:`5`
          (`self.CompletedQuest` (`self.QuestID`) :!label _label_2))
        (:`6`
          (goto _label_2)))))
  (return))

(fn `GetStartChatLog`
  (params (NPC_Prompts :type "Map of Name to String"))
  (returns (StartLog :type String))
  (set `self.Promps` NPC_Prompts)
  (return "You are a robotic worker, when the player announces that he wants help you say \"I would really like to build a wind turbine but I lost a propeller somewhere, could you help me?\". If after this sentence the player announces that he wants to complete the task, return \"Get quest\"."))

(fn `UserConstructionScript`)