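; Player character that talks to AI NPCs, collects pickups and earns gear that changes its gravity as quests progress.
; Front and surrounding colliders choose the current NPC and toggle name labels; holding Z records to that NPC, E takes the pickup.
; Postemp counts quest progress, granting a low-gravity head propeller (Wiatrak) or high-gravity back can (Puszka); Quest 1 also notifies its NPC.
; Tick pins gear to bones, spinning the propeller faster while falling.
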(event `self.ReceiveBeginPlay`
  (set `self.wiatrak speed` 200)
  (`SceneComponent.SetVisibility` (`self.smiglo`) false false)
  (`SceneComponent.SetVisibility` (`self.pucha`) false false)
  (bind _outactors (`GameplayStatics.GetAllActorsOfClass` "/Game/Blueprints/MyAI_NPC.MyAI_NPC_C"))
  (for _array_element _outactors
    (`BlueprintMapLibrary.Map_Add` (`self.NPC_Quest`) (`/Game/Blueprints/MyAI_NPC.QuestID` _array_element) _array_element)))

(event `PickUp`
  (params (NewParam :type "/Game/Blueprints/pickup Object Reference"))
  (set `self.CurrentPickUp` NewParam))

(event `self.ReceiveTick`
  (params (DeltaSeconds :type "Float (single-precision)"))
  (bind _smiglo (`self.smiglo`))
  (if (`self.puszka`)
    (`SceneComponent.K2_SetWorldLocation` (`self.pucha`) (`KismetMathLibrary.TransformLocation` (`SkinnedMeshComponent.GetBoneTransform` (`self.Mesh`) "spine_03" "RTS_World") (0.0 -20.0 5.0)) false false)
    (else
      (if (`NavMovementComponent.IsFalling` (`self.CharacterMovement`))
        (set `self.wiatrak speed` 1000)
        (else
          (set `self.wiatrak speed` 200)))
      (if (`self.wiatrak`)
        (`SceneComponent.K2_AddLocalRotation` _smiglo (`KismetMathLibrary.MakeRotator` 0.0 0.0 (* DeltaSeconds (`self.wiatrak speed`))) false false)
        (`SceneComponent.K2_SetWorldLocation` _smiglo (`KismetMathLibrary.TransformLocation` (`SkinnedMeshComponent.GetBoneTransform` (`self.Mesh`) "head" "RTS_World") (15.0 0.0 0.0)) false false)))))

(event `Key|E`
  (params (Key :type "Key Structure"))
  (bind _currentpickup (`self.CurrentPickUp`))
  (:`Pressed`
    (if (`KismetSystemLibrary.IsValid` _currentpickup)
      (if (`/Game/Blueprints/pickup.player near` _currentpickup)
        (`/Game/Blueprints/pickup.DestroyPickUp` _currentpickup)))))

(event `CheatWiatrak`
  (bind _currentnpc (`self.CurrentNPC`))
  (if (not (`self.wiatrak`))
    (`/Game/Blueprints/MyAI_NPC.AddSystemLog` _currentnpc (`BlueprintMapLibrary.Map_Find` (`/Game/Blueprints/MyAI_NPC.Promps` _currentnpc) "Cheat"))))

(event `Key|Z`
  (params (Key :type "Key Structure"))
  (bind _currentnpc (`self.CurrentNPC`))
  (bind _returnvalue (`KismetSystemLibrary.IsValid` _currentnpc))
  (:`Pressed`
    (if _returnvalue
      (`/Game/Blueprints/MyAI_NPC.StartRecording` _currentnpc)))
  (:`Released`
    (if _returnvalue
      (`/Game/Blueprints/MyAI_NPC.StopRecording` _currentnpc))))

(event `self.FrontCollider.OnComponentBeginOverlap`
  (params (OverlappedComponent :type "PrimitiveComponent Object Reference") (OtherActor :type "Actor Object Reference") (OtherComp :type "PrimitiveComponent Object Reference") (OtherBodyIndex :type Integer) (bFromSweep :type Boolean) (SweepResult :type "HitResult Structure (by ref)"))
  (bind _asmy_ai_npc (cast `/Game/Blueprints/MyAI_NPC` OtherActor))
  (bind _output_get (set `self.CurrentNPC` _asmy_ai_npc))
  (`/Game/Blueprints/MyAI_NPC.NameVisibllityOn` _output_get)
  (set `self.NPC_IsFront` true))

(event `self.FrontCollider.OnComponentEndOverlap`
  (params (OverlappedComponent :type "PrimitiveComponent Object Reference") (OtherActor :type "Actor Object Reference") (OtherComp :type "PrimitiveComponent Object Reference") (OtherBodyIndex :type Integer))
  (bind _asmy_ai_npc (cast `/Game/Blueprints/MyAI_NPC` OtherActor))
  (if (not (`PrimitiveComponent.IsOverlappingActor` (`self.AroundCollider`) _asmy_ai_npc))
    (`/Game/Blueprints/MyAI_NPC.NameVisibllityOff` _asmy_ai_npc)
    (set `self.CurrentNPC` null)
    (set `self.NPC_IsFront` false)))

(event `self.AroundCollider.OnComponentBeginOverlap`
  (params (OverlappedComponent :type "PrimitiveComponent Object Reference") (OtherActor :type "Actor Object Reference") (OtherComp :type "PrimitiveComponent Object Reference") (OtherBodyIndex :type Integer) (bFromSweep :type Boolean) (SweepResult :type "HitResult Structure (by ref)"))
  (if (not (`self.NPC_IsFront`))
    (bind _asmy_ai_npc (cast `/Game/Blueprints/MyAI_NPC` OtherActor))
    (`/Game/Blueprints/MyAI_NPC.NameVisibllityOn` _asmy_ai_npc)))

(event `self.AroundCollider.OnComponentEndOverlap`
  (params (OverlappedComponent :type "PrimitiveComponent Object Reference") (OtherActor :type "Actor Object Reference") (OtherComp :type "PrimitiveComponent Object Reference") (OtherBodyIndex :type Integer))
  (if (not (and (`self.NPC_IsFront`) (not (`KismetSystemLibrary.IsValid` (`self.CurrentNPC`)))))
    (bind _asmy_ai_npc (cast `/Game/Blueprints/MyAI_NPC` OtherActor))
    (`/Game/Blueprints/MyAI_NPC.NameVisibllityOff` _asmy_ai_npc)
    (set `self.CurrentNPC` null)))

(fn `Postemp`
  (params (`Nazwa Questa` :type Name))
  (bind _nazwaquesta (`self.NazwaQuesta`))
  (bind _nazwaquesta_2 (`self.NazwaQuesta`))
  (bind _postep (`self.Postep`))
  (bind (_value _returnvalue) (`BlueprintMapLibrary.Map_Find` (`self.NPC_Quest`) (`self.NazwaQuesta`)))
  (bind _instancequest (`/Game/Blueprints/MyAI_NPC.InstanceQuest` _value))
  (set `self.NazwaQuesta` `Nazwa Questa`)
  (`BlueprintMapLibrary.Map_Add` (`self.Postep`) _nazwaquesta_2 (+ (`BlueprintMapLibrary.Map_Find` _postep _nazwaquesta) 1))
  (switch `name` _nazwaquesta_2
    (:`Quest1`
      (if (== (`BlueprintMapLibrary.Map_Find` _postep _nazwaquesta) 1)
        (set `CharacterMovementComponent.GravityScale` 0.8 (`self.CharacterMovement`))
        (set `self.wiatrak` true)
        (`SceneComponent.SetVisibility` (`self.smiglo`) true false)
        (if _returnvalue
          (`/Game/Blueprints/MyAI_NPC.AddSystemLog` _value (`BlueprintMapLibrary.Map_Find` (`/Game/Blueprints/MyAI_NPC.Promps` _value) "Done Quest"))
          (if (`KismetSystemLibrary.IsValid` _instancequest)
            (set `QuestBase.bIsCompleted` true _instancequest)))))
    (:`Quest2`
      (if (== (`BlueprintMapLibrary.Map_Find` (`self.Postep`) "Quest2") 1)
        (set `CharacterMovementComponent.GravityScale` 3.5 (`self.CharacterMovement`))
        (`SceneComponent.SetVisibility` (`self.pucha`) true false)
        (set `self.puszka` true)))))

(fn `UserConstructionScript`)