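; Player character Blueprint for a quest game with voice-recorded AI NPCs and four quest items worn one at a time.
; Colliders track and label nearby NPCs, Z records to the current NPC, and E takes pickups.
; Postemp advances quests, shows items, changes gravity for some and notifies the mapped NPC; ItemsOff resets them.
; Tick pins items to bones, spins the propeller faster when falling, and drops the plant after prolonged falling.
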(event `self.ReceiveBeginPlay`
  (set `self.rownowaga` 12)
  (set `self.wiatrak speed` 200)
  (`SceneComponent.SetVisibility` (`self.smiglo`) false false)
  (`SceneComponent.SetVisibility` (`self.pucha`) false false)
  (`SceneComponent.SetVisibility` (`self.roslina`) false false)
  (`SceneComponent.SetVisibility` (`self.filtr`) false false)
  (bind _outactors (`GameplayStatics.GetAllActorsOfClass` "/Game/Blueprints/MyAI_NPC.MyAI_NPC_C"))
  (for _array_element _outactors
    (`BlueprintMapLibrary.Map_Add` (`self.NPC_Quest`) (`/Game/Blueprints/MyAI_NPC.QuestID` _array_element) _array_element)))

(event `PickUp`
  (params (NewParam :type "/Game/Blueprints/pickup Object Reference"))
  (set `self.CurrentPickUp` NewParam))

(event `self.ReceiveTick`
  (params (DeltaSeconds :type "Float (single-precision)"))
  (bind _smiglo (`self.smiglo`))
  (if (`self.filter`)
    (`SceneComponent.K2_SetWorldLocation` (`self.filtr`) (`KismetMathLibrary.TransformLocation` (`SkinnedMeshComponent.GetBoneTransform` (`self.Mesh`) "spine_03" "RTS_World") (0.0 -20.0 0.0)) false false)
    (elif (`self.roslinka`)
      (`SceneComponent.K2_SetWorldLocation` (`self.roslina`) (`KismetMathLibrary.TransformLocation` (`SkinnedMeshComponent.GetBoneTransform` (`self.Mesh`) "head" "RTS_World") (15.0 0.0 0.0)) false false)
      (if (`NavMovementComponent.IsFalling` (`self.CharacterMovement`))
        (`KismetSystemLibrary.Delay` 0.1)
        (set `self.rownowaga` (- (`self.rownowaga`) 1))
        (if (== (`self.rownowaga`) 0)
          (`BlueprintMapLibrary.Map_Add` (`self.Postep`) "Quest3")
          (`SceneComponent.SetVisibility` (`self.roslina`) false false)
          (set `self.roslinka` false)
          (set `self.eq` false))
        (else
          (set `self.rownowaga` 12)))
      (elif (`self.puszka`)
        (`SceneComponent.K2_SetWorldLocation` (`self.pucha`) (`KismetMathLibrary.TransformLocation` (`SkinnedMeshComponent.GetBoneTransform` (`self.Mesh`) "spine_03" "RTS_World") (0.0 -20.0 5.0)) false false)
        (elif (`self.wiatrak`)
          (if (`NavMovementComponent.IsFalling` (`self.CharacterMovement`))
            (set `self.wiatrak speed` 1000)
            (else
              (set `self.wiatrak speed` 200)))
          (`SceneComponent.K2_AddLocalRotation` _smiglo (`KismetMathLibrary.MakeRotator` 0.0 0.0 (* DeltaSeconds (`self.wiatrak speed`))) false false)
          (`SceneComponent.K2_SetWorldLocation` _smiglo (`KismetMathLibrary.TransformLocation` (`SkinnedMeshComponent.GetBoneTransform` (`self.Mesh`) "head" "RTS_World") (15.0 0.0 0.0)) false false))))))

(event `Key|E`
  (params (Key :type "Key Structure"))
  (bind _currentpickup (`self.CurrentPickUp`))
  (:`Pressed`
    (if (`self.eq`)
      _
      (elif (`KismetSystemLibrary.IsValid` _currentpickup)
        (if (`/Game/Blueprints/pickup.player near` _currentpickup)
          (`/Game/Blueprints/pickup.DestroyPickUp` _currentpickup)
          (set `self.eq` true))))))

(event `CheatWiatrak`
  (bind _currentnpc (`self.CurrentNPC`))
  (if (not (`self.wiatrak`))
    (`/Game/Blueprints/MyAI_NPC.AddSystemLog` _currentnpc (`BlueprintMapLibrary.Map_Find` (`/Game/Blueprints/MyAI_NPC.Promps` _currentnpc) "Cheat"))))

(event `Key|Z`
  (params (Key :type "Key Structure"))
  (bind _currentnpc (`self.CurrentNPC`))
  (bind _returnvalue (`KismetSystemLibrary.IsValid` _currentnpc))
  (:`Pressed`
    (if _returnvalue
      (`/Game/Blueprints/MyAI_NPC.StartRecording` _currentnpc)))
  (:`Released`
    (if _returnvalue
      (`/Game/Blueprints/MyAI_NPC.StopRecording` _currentnpc))))

(event `self.FrontCollider.OnComponentBeginOverlap`
  (params (OverlappedComponent :type "PrimitiveComponent Object Reference") (OtherActor :type "Actor Object Reference") (OtherComp :type "PrimitiveComponent Object Reference") (OtherBodyIndex :type Integer) (bFromSweep :type Boolean) (SweepResult :type "HitResult Structure (by ref)"))
  (bind _asmy_ai_npc (cast `/Game/Blueprints/MyAI_NPC` OtherActor))
  (bind _output_get (set `self.CurrentNPC` _asmy_ai_npc))
  (`/Game/Blueprints/MyAI_NPC.NameVisibllityOn` _output_get)
  (set `self.NPC_IsFront` true))

(event `self.FrontCollider.OnComponentEndOverlap`
  (params (OverlappedComponent :type "PrimitiveComponent Object Reference") (OtherActor :type "Actor Object Reference") (OtherComp :type "PrimitiveComponent Object Reference") (OtherBodyIndex :type Integer))
  (bind _asmy_ai_npc (cast `/Game/Blueprints/MyAI_NPC` OtherActor))
  (if (not (`PrimitiveComponent.IsOverlappingActor` (`self.AroundCollider`) _asmy_ai_npc))
    (`/Game/Blueprints/MyAI_NPC.NameVisibllityOff` _asmy_ai_npc)
    (set `self.CurrentNPC` null)
    (set `self.NPC_IsFront` false)))

(event `self.AroundCollider.OnComponentBeginOverlap`
  (params (OverlappedComponent :type "PrimitiveComponent Object Reference") (OtherActor :type "Actor Object Reference") (OtherComp :type "PrimitiveComponent Object Reference") (OtherBodyIndex :type Integer) (bFromSweep :type Boolean) (SweepResult :type "HitResult Structure (by ref)"))
  (if (not (`self.NPC_IsFront`))
    (bind _asmy_ai_npc (cast `/Game/Blueprints/MyAI_NPC` OtherActor))
    (`/Game/Blueprints/MyAI_NPC.NameVisibllityOn` _asmy_ai_npc)))

(event `self.AroundCollider.OnComponentEndOverlap`
  (params (OverlappedComponent :type "PrimitiveComponent Object Reference") (OtherActor :type "Actor Object Reference") (OtherComp :type "PrimitiveComponent Object Reference") (OtherBodyIndex :type Integer))
  (if (not (and (`self.NPC_IsFront`) (not (`KismetSystemLibrary.IsValid` (`self.CurrentNPC`)))))
    (bind _asmy_ai_npc (cast `/Game/Blueprints/MyAI_NPC` OtherActor))
    (`/Game/Blueprints/MyAI_NPC.NameVisibllityOff` _asmy_ai_npc)
    (set `self.CurrentNPC` null)))

(fn `CompletedQuest`
  (bind (_value _returnvalue) (`BlueprintMapLibrary.Map_Find` (`self.NPC_Quest`) (`self.NazwaQuesta`)))
  (bind _instancequest (`/Game/Blueprints/MyAI_NPC.InstanceQuest` _value))
  (if _returnvalue
    (`/Game/Blueprints/MyAI_NPC.AddSystemLog` _value (`BlueprintMapLibrary.Map_Find` (`/Game/Blueprints/MyAI_NPC.Promps` _value) "Done Quest"))
    (if (`KismetSystemLibrary.IsValid` _instancequest)
      (set `QuestBase.bIsCompleted` true _instancequest))))

(fn `ItemsOff`
  (params (QuestID :type Name))
  (switch `name` QuestID
    (:`Quest1`
      (set `self.wiatrak` false)
      (`SceneComponent.SetVisibility` (`self.smiglo`) false false))
    (:`Quest2`
      (set `self.puszka` false)
      (`SceneComponent.SetVisibility` (`self.pucha`) false false))
    (:`Quest3`
      (set `self.roslinka` false)
      (`SceneComponent.SetVisibility` (`self.roslina`) false false))
    (:`Quest4`
      (set `self.filter` false)
      (`SceneComponent.SetVisibility` (`self.filtr`) false false)))
  (`BlueprintMapLibrary.Map_Add` (`self.Postep`) QuestID)
  (set `self.eq` false))

(fn `Postemp`
  (params (`Nazwa Questa` :type Name))
  (bind _postep (`self.Postep`))
  (bind _postep_2 (`self.Postep`))
  (set `self.NazwaQuesta` `Nazwa Questa`)
  (`BlueprintMapLibrary.Map_Add` _postep_2 `Nazwa Questa` (+ (`BlueprintMapLibrary.Map_Find` _postep_2 `Nazwa Questa`) 1))
  (switch `name` `Nazwa Questa`
    (:`Quest1`
      ;[1 1 1] Smiglo
      (if (== (`BlueprintMapLibrary.Map_Find` _postep `Nazwa Questa`) 1)
        (set `CharacterMovementComponent.GravityScale` 0.8 (`self.CharacterMovement`))
        (set `self.wiatrak` true)
        (`SceneComponent.SetVisibility` (`self.smiglo`) true false)
        (`self.CompletedQuest`)))
    (:`Quest2`
      ;[1 1 1] Jedzenie
      (if (== (`BlueprintMapLibrary.Map_Find` _postep "Quest2") 1)
        (set `CharacterMovementComponent.GravityScale` 3.5 (`self.CharacterMovement`))
        (`SceneComponent.SetVisibility` (`self.pucha`) true false)
        (set `self.puszka` true)
        (`self.CompletedQuest`)))
    (:`Quest3`
      ;[1 1 1] Roslina
      (if (== (`BlueprintMapLibrary.Map_Find` _postep "Quest3") 1)
        (`SceneComponent.SetVisibility` (`self.roslina`) true false)
        (set `self.roslinka` true)
        (`self.CompletedQuest`)))
    (:`Quest4`
      ;[1 1 1] filtr
      (if (== (`BlueprintMapLibrary.Map_Find` _postep "Quest4") 1)
        (`SceneComponent.SetVisibility` (`self.filtr`) true false)
        (set `self.filter` true)
        (`self.CompletedQuest`)))))

(fn `UserConstructionScript`)